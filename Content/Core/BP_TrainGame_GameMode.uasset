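; Game mode for a train game that tracks whether track placement is active and collects track point locations.
; On BeginPlay it binds to a placing-tracks event, which updates the mode flag and sets or clears the current track node.
; When placement turns on, the node's world location is added uniquely to a point list, which GetTrackPoints exposes.
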(event Custom|On_PlacingTracksMode
  (params (TrackNode :type BP%20Track%20Node%20Object%20Reference) (PlacingTracks :type Boolean))
  (bind _output_get (Variables|Default|SetIsPlacingTracks PlacingTracks))
  (if _output_get
    (bind _output_get_2 (Variables|Default|SetTrackNode TrackNode))
    (CallFunction|AddVectortoTrackPoints _output_get_2)
    (else
      (Variables|Default|SetTrackNode 0))))

(event EventBeginPlay
  (EventDispatchers|BindEventtoPlacingTracksMode (EventDispatchers|CreateEvent :!event Custom|On_PlacingTracksMode)))

(fn ConstructionScript)

(fn AddVectortoTrackPoints
  (params (Target :type Actor%20Object%20Reference))
  (Utilities|Array|AddUnique (Variables|Default|GetTrackPoints) (Transformation|GetActorLocation Target)))

(fn GetTrackPoints
  (return (Variables|Default|GetTrackPoints)))