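; HUD for the train game that shows the main on-screen widget with the crosshair and opens a track options menu.
; On BeginPlay it adds W_HUD and binds to the player controller's button press and release events.
; Releasing the right mouse button recreates W_TrackOptions at the viewport center, then switches to UI-only input with a visible cursor.
; The press handler is empty.
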(event Custom|OnButtonReleased
  (params (Key :type Key%20Structure :default "None"))
  (bind _returnvalue (Game|GetPlayerController 0))
  (if (== Key "RightMouseButton")
    (bind _trackoptions (Variables|Default|GetTrackOptions)
      (:then
        (Widget|RemovefromParent _trackoptions))
      (:else
        _))
    (bind _returnvalue_2 (UserInterface|CreateWidget "/Game/UI/W_TrackOptions.W_TrackOptions_C" (Game|GetPlayerController 0)))
    (bind _output_get (Variables|Default|SetTrackOptions _returnvalue_2))
    (UserInterface|Viewport|AddtoViewport _output_get 0)
    (Class|UserWidget|SetPositioninViewport _output_get (CallFunction|GetViewportCenter) true)
    (Input|SetInputModeUIOnly _returnvalue 0 "DoNotLock")
    (Variables|/Script/Engine.PlayerController|SetbShowMouseCursor _returnvalue true)))

(event Custom|OnButtonPressed
  (params (Key :type Key%20Structure :default "None")))

(event EventBeginPlay
  (bind _returnvalue (Game|GetPlayerController 0))
  (bind _asbp_train_game_player_controller (Utilities|Casting|CastToBP_TrainGame_PlayerController _returnvalue))
  ;[1 1 1] Add crosshair to HUD
  (bind _returnvalue_2 (UserInterface|CreateWidget "/Game/UI/W_HUD.W_HUD_C" (Game|GetPlayerController 0)))
  (bind _output_get (Variables|Default|SetHUD _returnvalue_2))
  (UserInterface|Viewport|AddtoViewport _output_get 0)
  (EventDispatchers|BindEventtoButtonPressed _asbp_train_game_player_controller (EventDispatchers|CreateEvent :!event Custom|OnButtonReleased))
  (EventDispatchers|BindEventtoButtonReleased _asbp_train_game_player_controller (EventDispatchers|CreateEvent :!event Custom|OnButtonPressed)))

(fn ConstructionScript)

(fn GetViewportCenter
  (bind _returnvalue (Viewport|GetViewportSize))
  (return (Math|Vector2D|MakeVector2D (/ (.x _returnvalue) 2.0) (/ (.y _returnvalue) 2.0))))