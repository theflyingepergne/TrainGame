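; Player pawn for the train game that flies with axis input and mouse look, limiting vertical movement to a height band.
; Holding left click runs a looping timer that repeatedly line-traces and prints a debug message when it hits a BP_Track.
; The trace ends at the scaled forward vector without adding the pawn's location.
; Right click only prints a debug message.
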(event Custom|Trace
  (bind _outhit (Collision|LineTraceByChannel (Transformation|GetActorLocation) (* (Transformation|GetActorForwardVector) 1e+03) "TraceTypeQuery1" false 0 "ForDuration"))
  (Utilities|Casting|CastToBP_Track (.HitActor (Collision|BreakHitResult _outhit)))
  (Development|PrintString "Clicked on spline!" true true "(R=1.000000,G=0.863370,B=0.171760,A=1.000000)" 0.0))

(event Input|ActionEvents|InputActionLeftClick
  (params (Key :type Key%20Structure :default "None"))
  ;[1 1 1] Clicking input
  (:Pressed
    (Development|PrintString "Left clicked!")
    (bind _returnvalue (Utilities|Time|SetTimerbyEvent (delegate Custom|Trace) 0.01 true))
    (Variables|Default|SetTraceTimer _returnvalue))
  (:Released
    (Utilities|Time|ClearandInvalidateTimerbyHandle (Variables|Default|GetTraceTimer))))

(event Input|ActionEvents|InputActionRightClick
  (params (Key :type Key%20Structure :default "None"))
  ;[1 1 1] Clicking input
  (:Pressed
    (Development|PrintString "RightClicked")))

(event Input|AxisEvents|InputAxisMouseRight
  (params (AxisValue :type Float%20%28single-precision%29))
  ;[1 1 1] Mouse look around
  (Pawn|Input|AddControllerYawInput AxisValue))

(event Input|AxisEvents|InputAxisMoveFoward
  (params (AxisValue :type Float%20%28single-precision%29))
  (bind _returnvalue (Transformation|GetActorForwardVector))
  ;[1 1 1] Moving left, right, foward, backward
  (Pawn|Input|AddMovementInput (Math|Vector|MakeVector (.x _returnvalue) (.y _returnvalue) 0.0) AxisValue false))

(event Input|AxisEvents|InputAxisMoveBackward
  (params (AxisValue :type Float%20%28single-precision%29))
  (bind _returnvalue (Transformation|GetActorForwardVector))
  ;[1 1 1] Moving left, right, foward, backward
  (Pawn|Input|AddMovementInput (Math|Vector|MakeVector (.x _returnvalue) (.y _returnvalue) 0.0) AxisValue false))

(event Input|AxisEvents|InputAxisMoveRight
  (params (AxisValue :type Float%20%28single-precision%29))
  ;[1 1 1] Moving left, right, foward, backward
  (Pawn|Input|AddMovementInput (Transformation|GetActorRightVector) AxisValue false))

(event Input|AxisEvents|InputAxisMoveLeft
  (params (AxisValue :type Float%20%28single-precision%29))
  ;[1 1 1] Moving left, right, foward, backward
  (Pawn|Input|AddMovementInput (Transformation|GetActorRightVector) AxisValue false))

(event Input|AxisEvents|InputAxisMouseForward
  (params (AxisValue :type Float%20%28single-precision%29))
  ;[1 1 1] Mouse look around
  (Pawn|Input|AddControllerPitchInput AxisValue))

(event Input|AxisEvents|InputAxisMoveUp
  (params (AxisValue :type Float%20%28single-precision%29))
  ;[1 1 1] Move up and down (clamped)
  (if (< (.z (Transformation|GetActorLocation)) 5e+02)
    (Pawn|Input|AddMovementInput "0, 0,1.000000" AxisValue false)))

(event Input|AxisEvents|InputAxisMoveDown
  (params (AxisValue :type Float%20%28single-precision%29))
  ;[1 1 1] Move up and down (clamped)
  (if (> (.z (Transformation|GetActorLocation)) 1e+02)
    (Pawn|Input|AddMovementInput "0, 0,1.000000" AxisValue false)))

(fn ConstructionScript)