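; BP_Station is a train station actor that tracks the trains currently at it and shows its name on a text component.
; Its trigger box adds each overlapping BP_Train to a list and notifies that train, passing itself as the station.
; A LeaveStation event removes a given train from the list, and the construction script applies the configured name text.
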(event OnComponentBeginOverlap(BoxTrigger)
  (params (OverlappedComponent :type Primitive%20Component%20Object%20Reference) (OtherActor :type Actor%20Object%20Reference) (OtherComp :type Primitive%20Component%20Object%20Reference) (OtherBodyIndex :type Integer) (bFromSweep :type Boolean) (SweepResult :type Hit%20Result%20Structure%20%28by%20ref%29))
  (Development|PrintString "Train approached station" true true "(R=1.000000,G=0.201579,B=0.000000,A=1.000000)")
  (bind _asbp_train (Utilities|Casting|CastToBP_Train OtherActor))
  (Utilities|Array|Add (Variables|Default|GetTrainsAtStation) _asbp_train)
  (Class|BPITrainTrackInterface|HandleTrainatStation(Message) _asbp_train self))

(event EventLeaveStation
  (params (Train :type BP%20Train%20Object%20Reference))
  (bind _returnvalue (Utilities|Array|RemoveItem (Variables|Default|GetTrainsAtStation) Train))
  (if _returnvalue
    (Development|PrintString "removed" true true "(R=1.000000,G=0.201579,B=0.000000,A=1.000000)")
    (else
      (Development|PrintString "nothing to remove" true true "(R=1.000000,G=0.201579,B=0.000000,A=1.000000)"))))

(fn ConstructionScript
  (Rendering|Components|TextRender|SetText (Variables|Default|GetStationName) (Variables|Default|GetStationName_Text)))