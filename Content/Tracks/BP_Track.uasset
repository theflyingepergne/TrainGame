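; Spline-based train track that builds its own track geometry and spawns a train to run along it.
; The construction script tiles spline meshes in sections sized from the mesh bounds, adding an optional start terminus and an end child actor.
; On BeginPlay it spawns the train with carriage-offset start and end distances.
; UpdatedTimeline maps an alpha to spline position, flipping the train when travelling backward, while helper functions report arrival at either end.
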(event Custom|SpawnTrain
  (bind _distance_along_spline (CallFunction|GetTrainStartTransform))
  (bind _returnvalue (Game|SpawnActorfromClass (Variables|Default|GetTrainType) (Spline|GetTransformatDistanceAlongSpline (Variables|Default|GetSpline) _distance_along_spline "World" false) "Undefined" 0 self (Variables|Default|GetNum%20Carriages) _distance_along_spline (CallFunction|GetTrainEndTransform) 0)) ; Spawn train on track, supply information
  (Variables|Default|SetAttachedTrain _returnvalue))

(event EventUpdatedTimeline
  (params (Direction :type ETimelineDirection%20Enum :default "Forward") (PointAlongSpline :type Float%20%28double-precision%29) (TrainToMove :type Actor%20Object%20Reference))
  (Variables|Default|SetDirection Direction)
  (CallFunction|UpdateTrainPositiononTrack PointAlongSpline TrainToMove) ; Update train position on track
)

(event EventBeginPlay
  (CallFunction|SpawnTrain)
  (Development|PrintString (Utilities|String|Append "Track length for" (Utilities|GetDisplayName self) " = " (Utilities|String|ToString(Float) (Spline|GetSplineLength (Variables|Default|GetSpline)))) true true "(R=0.073477,G=0.000000,B=0.182292,A=1.000000)" 5.0))

(fn ConstructionScript
  (bind _trackmesh (Variables|PreConstruct|GetTrackMesh))
  (bind _spline (Variables|Default|GetSpline))
  (bind _spline_2 (Variables|Default|GetSpline))
  (bind _returnvalue (StaticMesh|GetBoundingBox _trackmesh))
  (bind _returnvalue_2 (Spline|GetTransformatSplinePoint _spline_2 0 "Local" false))
  (bind (_min _max) (Utilities|Struct|BreakBox _returnvalue))
  (bind _returnvalue_3 (AddComponent|AddTextRenderComponent false (Math|Transform|MakeTransform "0, 0,100.000000" "0, 0, 0" "1.000000,1.000000,1.000000")))
  (Rendering|Components|TextRender|SetText _returnvalue_3 (Utilities|Text|ToText(String) (Utilities|String|Append (Utilities|GetDisplayName self) ", Length = " (Utilities|String|ToString(Integer) (Math|Float|Truncate (Spline|GetSplineLength (Variables|Default|GetSpline)))))))
  (Class|SplineComponent|SetDrawDebug (Variables|Default|GetSpline) true)
  (if (Variables|PreConstruct|GetAddTrackTerminus)
    ;[1 1 1] Add a track terminus at the beginning (if you want). True  by default
    (AddComponent|AddChildActorComponent false (Math|Transform|MakeTransform (Math|Vector|MakeVector (- (.x (.location _returnvalue_2)) (Variables|PreConstruct|GetSectionLengthCoef)) (.y (.location _returnvalue_2)) (.z (.location _returnvalue_2))) (.rotation _returnvalue_2) (.scale _returnvalue_2))))
  ;[1 1 1] Calculate 1 SectiongLength
  (Variables|PreConstruct|SetSectionLength (* (.x (Transformation|GetActorScale3D)) (Variables|PreConstruct|GetSectionLengthCoef)))
  ;[1 1 1] Determine how many SectionLengths can fit on the spline
  (for _index (range 0 (- (Math|Float|Truncate (/ (Spline|GetSplineLength (Variables|Default|GetSpline)) (Variables|PreConstruct|GetSectionLength))) 1))
    (Variables|PreConstruct|SetCurrentIndex _index)
    ;[1 1 1] Add spline mesh component and set the static mesh
    (bind _returnvalue_4 (AddComponent|AddSplineMeshComponent false))
    (bind _output_get (Variables|Default|SetSplineMeshComponent _returnvalue_4))
    (Components|StaticMesh|SetStaticMesh _output_get (Variables|PreConstruct|GetTrackMesh))
    ;[1 1 1] Use static mesh bounds to calculate SectionLengthCoef (after setting manually once)
    (Variables|PreConstruct|SetSectionLengthCoef (- (.x _max) (.x _min)))
    ;[1 1 1] Calculate spline mesh start and end
    (SplineMesh|SetStartandEnd (Variables|Default|GetSplineMeshComponent) (Spline|GetLocationatDistanceAlongSpline (Variables|Default|GetSpline) (* (Variables|PreConstruct|GetCurrentIndex) (Variables|PreConstruct|GetSectionLength)) "Local") (Math|Vector|ClampVectorSize (Spline|GetTangentatDistanceAlongSpline (Variables|Default|GetSpline) (* (Variables|PreConstruct|GetCurrentIndex) (Variables|PreConstruct|GetSectionLength)) "Local") (Variables|PreConstruct|GetSectionLength) (Variables|PreConstruct|GetSectionLength)) (Spline|GetLocationatDistanceAlongSpline (Variables|Default|GetSpline) (* (+ (Variables|PreConstruct|GetCurrentIndex) 1) (Variables|PreConstruct|GetSectionLength)) "Local") (Math|Vector|ClampVectorSize (Spline|GetTangentatDistanceAlongSpline (Variables|Default|GetSpline) (* (+ (Variables|PreConstruct|GetCurrentIndex) 1) (Variables|PreConstruct|GetSectionLength)) "Local") (Variables|PreConstruct|GetSectionLength) (Variables|PreConstruct|GetSectionLength)) true :!class /Script/Engine.SplineMeshComponent)
    ;[1 1 1] Set Spline Mesh collision
    (Collision|SetCollisionEnabled (Variables|Default|GetSplineMeshComponent) (Variables|PreConstruct|GetCollisionEnabledType))
    (Collision|SetCollisionResponsetoAllChannels (Variables|Default|GetSplineMeshComponent) (Variables|PreConstruct|GetCollisionResponseType)))
  ;[1 1 1] Add an extra bit of track on at the end - TrackTerminus if spline is not closed
  (if (Variables|PreConstruct|GetAddTrackTerminus)
    (AddComponent|AddChildActorComponent false (Math|Transform|MakeTransform (+ (Spline|GetLocationatDistanceAlongSpline _spline (* (+ (Variables|PreConstruct|GetCurrentIndex) 1) (Variables|PreConstruct|GetSectionLength)) "Local") (* (Math|Vector|GetForwardVector (Spline|GetRotationatDistanceAlongSpline _spline (* (+ (Variables|PreConstruct|GetCurrentIndex) 1) (Variables|PreConstruct|GetSectionLength)) "Local")) (Variables|PreConstruct|GetSectionLength))) (Math|Rotator|MakeRotator (.Roll (Math|Rotator|BreakRotator (Spline|GetRotationatDistanceAlongSpline _spline (* (+ (Variables|PreConstruct|GetCurrentIndex) 1) (Variables|PreConstruct|GetSectionLength)) "Local"))) (.Pitch (Math|Rotator|BreakRotator (Spline|GetRotationatDistanceAlongSpline _spline (* (+ (Variables|PreConstruct|GetCurrentIndex) 1) (Variables|PreConstruct|GetSectionLength)) "Local"))) (- (.Yaw (Math|Rotator|BreakRotator (Spline|GetRotationatDistanceAlongSpline _spline (* (+ (Variables|PreConstruct|GetCurrentIndex) 1) (Variables|PreConstruct|GetSectionLength)) "Local"))) 1.8e+02))))
    (else
      (AddComponent|AddChildActorComponent false (Math|Transform|MakeTransform (+ (Spline|GetLocationatDistanceAlongSpline _spline (* (+ (Variables|PreConstruct|GetCurrentIndex) 1) (Variables|PreConstruct|GetSectionLength)) "Local") (* (Math|Vector|GetForwardVector (Spline|GetRotationatDistanceAlongSpline _spline (* (+ (Variables|PreConstruct|GetCurrentIndex) 1) (Variables|PreConstruct|GetSectionLength)) "Local")) (Variables|PreConstruct|GetSectionLength))) (Math|Rotator|MakeRotator (.Roll (Math|Rotator|BreakRotator (Spline|GetRotationatDistanceAlongSpline _spline (* (+ (Variables|PreConstruct|GetCurrentIndex) 1) (Variables|PreConstruct|GetSectionLength)) "Local"))) (.Pitch (Math|Rotator|BreakRotator (Spline|GetRotationatDistanceAlongSpline _spline (* (+ (Variables|PreConstruct|GetCurrentIndex) 1) (Variables|PreConstruct|GetSectionLength)) "Local"))) (- (.Yaw (Math|Rotator|BreakRotator (Spline|GetRotationatDistanceAlongSpline _spline (* (+ (Variables|PreConstruct|GetCurrentIndex) 1) (Variables|PreConstruct|GetSectionLength)) "Local"))) 1.8e+02)))))))

(fn GetIsTrainatTrackEnd
  (bind _attachedtrain (CallFunction|GetAttachedTrain))
  (bind _returnvalue (Transformation|GetActorLocation _attachedtrain))
  (return (or (Class|KismetMathLibrary|EqualExactlyVectorVector (Spline|GetLocationatSplinePoint (Variables|Default|GetSpline) (CallFunction|GetLastSplineIndex) "World") _returnvalue) (Class|KismetMathLibrary|EqualExactlyVectorVector _returnvalue (Spline|GetLocationatDistanceAlongSpline (Variables|Default|GetSpline) (CallFunction|GetTrainEndTransform) "World")))))

(fn GetAttachedTrain
  (return (Variables|Default|GetAttachedTrain)))

(fn UpdateTrainPositiononTrack
  (params (PointAlongSpline :type Float%20%28double-precision%29) (TrainToMove :type Actor%20Object%20Reference))
  (bind _direction (Variables|Default|GetDirection))
  (bind _spline (Variables|Default|GetSpline))
  (bind _spline_2 (Variables|Default|GetSpline))
  (bind _returnvalue (Spline|GetSplineLength _spline_2))
  (bind _returnvalue_2 (Math|Float|Lerp 0.0 _returnvalue PointAlongSpline))
  (bind _returnvalue_3 (Spline|GetRotationatDistanceAlongSpline _spline _returnvalue_2 "World"))
  ;[1 1 1] Update the train's position and rotation along the track. If the train is on its return journey, rotate it 180 degrees.
  (Transformation|SetActorTransform TrainToMove (Math|Transform|MakeTransform (Spline|GetLocationatDistanceAlongSpline _spline _returnvalue_2 "World") (Math|Rotator|MakeRotator (.roll _returnvalue_3) (* (.pitch _returnvalue_3) (Utilities|Select :Index _direction :Forward 1.0 :Backward -1.0)) (- (.yaw _returnvalue_3) (Utilities|Select :Index _direction :Forward 0.0 :Backward 1.8e+02))) "1.000000,1.000000,1.000000")))

(fn GetIsTrainatTrackBeginning
  (bind _attachedtrain (CallFunction|GetAttachedTrain))
  (bind _returnvalue (Transformation|GetActorLocation _attachedtrain))
  (return (or (Class|KismetMathLibrary|EqualExactlyVectorVector (Spline|GetLocationatSplinePoint (Variables|Default|GetSpline) 0 "World") _returnvalue) (Class|KismetMathLibrary|EqualExactlyVectorVector _returnvalue (Spline|GetLocationatDistanceAlongSpline (Variables|Default|GetSpline) (CallFunction|GetTrainStartTransform) "World")))))

(fn GetLastSplineIndex
  (return (- (Spline|GetNumberOfSplinePoints (Variables|Default|GetSpline)) 1)))

(fn GetTrainStartTransform
  (return (Math|Conversions|ToFloat(Integer) (* (Variables|Default|GetNum%20Carriages) 300))))

(fn GetTrainEndTransform
  (return (- (Spline|GetSplineLength (Variables|Default|GetSpline)) (Math|Conversions|ToFloat(Integer) (* (Variables|Default|GetNum%20Carriages) 300)))))