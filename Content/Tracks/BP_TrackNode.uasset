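; Track node actor for a train game, laying track as spline mesh segments along a spline.
; The construction script adds one spline mesh per whole SectionLength of spline, with tangents clamped to that length.
; On BeginPlay during track placement, it appends its location to the game mode's TrackNode spline and prints debug stats.
; BeginPlay also sets spline points from the game mode's track points, without rebuilding the meshes itself.
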(event EventBeginPlay
  (if (Variables|/Game/Core/BP_TrainGame_GameMode.BP_TrainGame_GameMode_C|GetIsPlacingTracks (CallFunction|GetTrainGameGameMode))
    (bind _output_get (Variables|Default|SetSpline (Variables|Default|GetSpline (Variables|/Game/Core/BP_TrainGame_GameMode.BP_TrainGame_GameMode_C|GetTrackNode (CallFunction|GetTrainGameGameMode)))))
    (Class|SplineComponent|AddPoint _output_get (Utilities|Struct|MakeSplinePoint 1.0 (Transformation|GetActorLocation)) true)
    (Development|PrintString (Utilities|String|ToString(Integer) (Spline|GetNumberOfSplinePoints _output_get)))
    (Development|PrintString (Utilities|String|ToString(Float) (Spline|GetSplineLength (Variables|Default|GetSpline))) true true "(R=1.000000,G=0.145583,B=0.000000,A=1.000000)"))
  (Spline|SetSplinePoints (Variables|Default|GetSpline) (Default|GetTrackPoints (CallFunction|GetTrainGameGameMode)) "Local" true))

(fn ConstructionScript
  (bind _sectionlength (LocalVariables|GetSectionLength))
  (bind _sectionlength_2 (LocalVariables|GetSectionLength))
  (for _index (range 0 (- (Math|Float|Truncate (/ (Spline|GetSplineLength (Variables|Default|GetSpline)) (LocalVariables|GetSectionLength))) 1))
    (LocalVariables|SetCurrentIndex _index)
    (bind _returnvalue (AddComponent|AddSplineMeshComponent false))
    (LocalVariables|SetSplineMeshComponent _returnvalue)
    (SplineMesh|SetStartandEnd (LocalVariables|GetSplineMeshComponent) (Spline|GetLocationatDistanceAlongSpline (Variables|Default|GetSpline) (* (LocalVariables|GetCurrentIndex) (LocalVariables|GetSectionLength)) "Local") (Math|Vector|ClampVectorSize (Spline|GetTangentatDistanceAlongSpline (Variables|Default|GetSpline) (* (LocalVariables|GetCurrentIndex) (LocalVariables|GetSectionLength)) "Local") _sectionlength _sectionlength) (Spline|GetLocationatDistanceAlongSpline (Variables|Default|GetSpline) (* (+ (LocalVariables|GetCurrentIndex) 1) (LocalVariables|GetSectionLength)) "Local") (Math|Vector|ClampVectorSize (Spline|GetTangentatDistanceAlongSpline (Variables|Default|GetSpline) (* (+ (LocalVariables|GetCurrentIndex) 1) (LocalVariables|GetSectionLength)) "Local") _sectionlength_2 _sectionlength_2) true :!class /Script/Engine.SplineMeshComponent)))