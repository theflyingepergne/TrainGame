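; Train actor that travels along an attached track's spline, toggling between moving and stopped with steam and audio effects.
; A timeline, rate-scaled by speed over spline length, sends its position and direction to the track, which is told which train to move.
; MoveTrain picks forward or reverse from track-end state.
; Station arrivals sound the horn and pause the train on a timer before it departs and notifies the station.
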(event Custom|RestartLoop
  (bind _attachedtrack (CallFunction|GetAttachedTrack))
  (bind (_direction _pointalongspline__0_1_) (Timeline|MoveAlongTrack PlayFromStart)
    (:Update
      (bind _output_get (Variables|Default|SetDirection _direction))
      ;[1 1 1] Send timeline info to track
      (Default|UpdatedTimeline _attachedtrack _output_get self _pointalongspline__0_1_))
    (:Finished
      ;[1 1 1] If spline is closed, play from start. Else, stop train
      (if (Class|SplineComponent|IsClosedLoop (Variables|/Game/Tracks/BP_Track.BP_Track_C|GetSpline _attachedtrack))
        (CallFunction|RestartLoop)
        (else
          (CallFunction|StopTrain))))))

(event EventHandleTrainatStation
  (params (Station :type BP%20Station%20Object%20Reference))
  (Variables|Default|SetStation Station)
  (Development|PrintString "Train arrived at station" true true "(R=1.000000,G=0.201579,B=0.000000,A=1.000000)")
  ;[1 1 1] Play horn when train arrives at station
  (Effects|Components|ParticleSystem|SetIntParameter (Variables|Default|GetTrainAudio) "PlayHorn" 1)
  ;[1 1 1] Stop train when arriving at station
  (Variables|Default|SetIsTrainAtStation true)
  (CallFunction|StopTrain self)
  (Timeline|TimeAtStation PlayFromStart ; Wait at the station for a while...
    (:Finished
      ;[1 1 1] Move train away from station, tell the station the train has left, resume typical train noises uwu
      (CallFunction|MoveTrain)
      (Class|BPIStationInterface|LeaveStation(Message) (CallFunction|GetStation) self)
      (Variables|Default|SetStation 0)
      (Variables|Default|SetIsTrainAtStation false)
      (Effects|Components|ParticleSystem|SetIntParameter (Variables|Default|GetTrainAudio) "PlayHorn" 0))))

(event EventBeginPlay)

(event EventStopTrain
  (params (Train :type BP%20Train%20Object%20Reference))
  (bind _trainaudio (Variables|Default|GetTrainAudio))
  (bind _audiofadeduration (Variables|Default|GetAudioFadeDuration))
  ;[1 1 1] Stop train, stop steam
  (Audio|Components|Audio|Stop (Variables|Default|GetMoveAlongTrack))
  (Variables|Default|SetTrainMoving false)
  (bind _steam (Variables|Default|GetSteam)
    (:then
      (Components|Activation|Deactivate _steam)
      ;[1 1 1] Stop audio if train stops anywhere other than at station
      (if (not (Variables|Default|GetIsTrainAtStation))
        (Audio|Components|Audio|FadeOut _trainaudio _audiofadeduration 0.0 "Linear" :!class /Script/Engine.AudioComponent)
        (Utilities|FlowControl|Delay _audiofadeduration)
        (Components|Activation|Deactivate _trainaudio)
        (else
          (Development|PrintString "Train stopped at station" true true "(R=1.000000,G=0.201579,B=0.000000,A=1.000000)"))))
    (:else)))

(event EventMoveTrain
  (bind _attachedtrack (CallFunction|GetAttachedTrack))
  ;[1 1 1] If the train is moving, stop it. Else, begin the moving process 👀
  (if (not (Variables|Default|GetTrainMoving))
    (Variables|Default|SetTrainMoving true)
    ;[1 1 1] Activate components
    (bind _steam (Variables|Default|GetSteam)
      (:then
        (Components|Activation|Activate _steam false)
        (Audio|Components|Audio|FadeIn (Variables|Default|GetTrainAudio) (Variables|Default|GetAudioFadeDuration) 1.0 0.0 "Linear" :!class /Script/Engine.AudioComponent)
        (CallFunction|SetTrainTravelSpeed) ; Use TrainSpeed to set train speed
        ;[1 1 1] Train direction and distance along track logic
        (if (or (not (Default|GetIsTrainatTrackEnd (CallFunction|GetAttachedTrack))) (Class|SplineComponent|IsClosedLoop (Variables|/Game/Tracks/BP_Track.BP_Track_C|GetSpline (CallFunction|GetAttachedTrack))))
          (Variables|Default|SetTrainAtTrackEnd false)
          (switch Utilities|FlowControl|Switch|SwitchonETimelineDirection (Variables|Default|GetDirection)
            (:Forward
              (if (Default|GetIsTrainatTrackBeginning (CallFunction|GetAttachedTrack))
                (Utilities|FlowControl|Sequence :!label _label ; Set the start time THEN play
                  (:then_0
                    (Variables|Default|SetDirection "Forward")
                    (bind (_direction _pointalongspline__0_1_) (Timeline|MoveAlongTrack SetNewTime)
                      (:Update
                        (bind _output_get (Variables|Default|SetDirection _direction))
                        ;[1 1 1] Send timeline info to track
                        (Default|UpdatedTimeline _attachedtrack _output_get self _pointalongspline__0_1_))
                      (:Finished
                        ;[1 1 1] If spline is closed, play from start. Else, stop train
                        (if (Class|SplineComponent|IsClosedLoop (Variables|/Game/Tracks/BP_Track.BP_Track_C|GetSpline _attachedtrack))
                          (CallFunction|RestartLoop)
                          (else
                            (CallFunction|StopTrain))))))
                  (:then_1
                    (Timeline|MoveAlongTrack Play)))
                (else
                  (Timeline|MoveAlongTrack Play))))
            (:Backward
              (if (Default|GetIsTrainatTrackBeginning (CallFunction|GetAttachedTrack))
                (goto _label)
                (else
                  (Timeline|MoveAlongTrack Reverse)))))
          (else
            (Variables|Default|SetTrainAtTrackEnd true)
            (Utilities|FlowControl|Sequence ; Set the start time THEN play
              (:then_0
                (Variables|Default|SetDirection "Backward")
                (Timeline|MoveAlongTrack SetNewTime))
              (:then_1
                (Timeline|MoveAlongTrack Reverse))))))
      (:else))
    (else
      (CallFunction|StopTrain))))

(fn ConstructionScript
  ;[1 1 1] Debuggering
  (bind _returnvalue (AddComponent|AddTextRenderComponent false (Math|Transform|MakeTransform "0, 0,150.000000" "0, 0, 0" "1.000000,1.000000,1.000000")))
  (bind _output_get (Variables|Default|SetName_TextRender _returnvalue))
  (Rendering|Components|TextRender|SetText _output_get (Utilities|Text|ToText(String) (Utilities|GetDisplayName self))))

(fn GetAttachedTrack
  (return (Variables|SetOnSpawn|GetAttachedTrack)))

(fn GetTrainMesh
  (return (Variables|Default|GetVehicleMesh)))

(fn GetTrainSpeed
  (return (Variables|SetOnSpawn|GetTrainSpeed)))

(fn GetStation
  (return (Variables|Default|GetStation)))

(fn GetIsTrainatStation
  (return (Variables|Default|GetIsTrainAtStation)))

(fn SetTrainTravelSpeed
  (Components|Timeline|SetPlayRate (Variables|Default|GetMoveAlongTrack) (/ (CallFunction|GetTrainSpeed) (Spline|GetSplineLength (Variables|/Game/Tracks/BP_Track.BP_Track_C|GetSpline (CallFunction|GetAttachedTrack))))))

(fn GetNumCarriagestoSpawn
  (return (- (Variables|Carriage|GetTrainIndex) 1)))

(fn GetTrainStartTime
  (bind _trainstartpoint (Variables|SetOnSpawn|GetTrainStartPoint))
  (return (Math|Float|SelectFloat 0.0 (/ 1.0 (/ (Spline|GetSplineLength (Variables|/Game/Tracks/BP_Track.BP_Track_C|GetSpline (CallFunction|GetAttachedTrack))) _trainstartpoint)) (== _trainstartpoint 0.0))))

(fn GetTrainEndTime
  (return (Math|Float|SelectFloat 1.0 (/ 1.0 (/ (Spline|GetSplineLength (Variables|/Game/Tracks/BP_Track.BP_Track_C|GetSpline (CallFunction|GetAttachedTrack))) (Variables|SetOnSpawn|GetTrainReturnPoint))) (Class|SplineComponent|IsClosedLoop (Variables|/Game/Tracks/BP_Track.BP_Track_C|GetSpline (CallFunction|GetAttachedTrack))))))